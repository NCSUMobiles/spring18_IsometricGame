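; Cat pickup actor that sends the player back to the Lobby level when touched.
; A Float timeline started on BeginPlay moves the root vertically by adding its track value to the current Z on each update.
; Actor overlap and Box overlap handlers duplicate the exit sequence: camera fade, short delay, then level load.
; The Box path filters by casting to PlayerCharacter and also prints a red debug string.
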(event `self.ReceiveBeginPlay`
  (bind _returnvalue (`SceneComponent.GetRelativeTransform` (`self.DefaultSceneRoot`)))
  (bind (_direction _newtrack_0) (`Timeline|Float` :!via `PlayFromStart`)
    (:`Update`
      (`SceneComponent.K2_SetRelativeLocation` (`self.DefaultSceneRoot`) (`KismetMathLibrary.MakeVector` (.x (.location _returnvalue)) (.y (.location _returnvalue)) (+ (.z (.location _returnvalue)) _newtrack_0)) false false))))

(event `self.ReceiveActorBeginOverlap`
  (params (OtherActor :type "Actor Object Reference"))
  (if (== null (`GameplayStatics.GetPlayerCharacter` 0))
    (`PlayerCameraManager.StartCameraFade` :`self` (`GameplayStatics.GetPlayerCameraManager` 0) :`ToAlpha` 1.0 :`Duration` 2.0 :`bHoldWhenFinished` true)
    (`KismetSystemLibrary.Delay` 2.0)
    (`GameplayStatics.OpenLevel` "Lobby")))

(event `self.Box.OnComponentBeginOverlap`
  (params (OverlappedComponent :type "PrimitiveComponent Object Reference") (OtherActor :type "Actor Object Reference") (OtherComp :type "PrimitiveComponent Object Reference") (OtherBodyIndex :type Integer) (bFromSweep :type Boolean) (SweepResult :type "HitResult Structure (by ref)"))
  (bind _asplayer_character (cast `PlayerCharacter` OtherActor))
  (if (== OtherActor _asplayer_character)
    (`KismetSystemLibrary.PrintString` "Hello" true true (struct :`R` 1.0 :`G` 0.08125 :`B` 0.08125 :`A` 1.0))
    (`PlayerCameraManager.StartCameraFade` :`self` (`GameplayStatics.GetPlayerCameraManager` 0) :`ToAlpha` 1.0 :`Duration` 2.0 :`bHoldWhenFinished` true)
    (`KismetSystemLibrary.Delay` 2.0)
    (`GameplayStatics.OpenLevel` "Lobby")))

(fn `UserConstructionScript`)