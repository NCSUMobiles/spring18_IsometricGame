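; Player character Blueprint that provides a camera fade effect on the first player camera manager.
; BeginPlay and the FadeCameraEffect event share one chain that logs a message, branches on InOrOut and starts a camera fade over FadeDuration.
; An optional delay, set by HasDelay and DelayDuration, ends the chain with nothing wired after it.
; Tick, overlap and the construction script are empty.
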(event `self.ReceiveBeginPlay`
  (bind _returnvalue (`GameplayStatics.GetPlayerCameraManager` 0))
  (`VisualLoggerKismetLibrary.LogText` "in character fade" :!label _label)
  ;[1 1 1] Comment
  (if (stale `self.FadeCameraEffect` inOrOut)
    (`PlayerCameraManager.StartCameraFade` :`self` _returnvalue :`Duration` (`KismetMathLibrary.Conv_IntToDouble` (stale `self.FadeCameraEffect` fadeDuration)))
    (else
      (`PlayerCameraManager.StartCameraFade` :`self` _returnvalue :`Duration` (`KismetMathLibrary.Conv_IntToDouble` (stale `self.FadeCameraEffect` fadeDuration)))))
  (if (stale `self.FadeCameraEffect` hasDelay)
    (`KismetSystemLibrary.Delay` (`KismetMathLibrary.Conv_IntToDouble` (stale `self.FadeCameraEffect` delayDuration)))))

(event `self.FadeCameraEffect`
  (params (inOrOut :type Boolean) (fadeDuration :type Integer) (hasDelay :type Boolean) (delayDuration :type Integer))
  (goto _label))

(fn `UserConstructionScript`)