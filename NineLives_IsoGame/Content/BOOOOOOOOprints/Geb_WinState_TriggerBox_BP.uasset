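; Trigger box that serves as a puzzle win condition, counting special DraggableBlocks inside its collision.
; Overlap begin increments WinCount and overlap end decrements it, with debug prints for each change.
; When the count reaches four, it prints a winner message, activates the target Block and, after a short delay, makes the target cat pickup's sprite visible.
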(event `self.CollisionComponent.OnComponentBeginOverlap`
  (params (OverlappedComponent :type "PrimitiveComponent Object Reference") (OtherActor :type "Actor Object Reference") (OtherComp :type "PrimitiveComponent Object Reference") (OtherBodyIndex :type Integer) (bFromSweep :type Boolean) (SweepResult :type "HitResult Structure (by ref)"))
  (bind _wincount (`self.WinCount`))
  (bind _asdraggable_block (cast `DraggableBlock` OtherActor))
  (if (== OtherActor _asdraggable_block)
    (if (`DraggableBlock.isSpecial` _asdraggable_block)
      (`/Engine/EditorBlueprintResources/StandardMacros.IncrementInt` _wincount
        (:`  `
          (`KismetSystemLibrary.PrintString` "+1 ")
          (if (== _wincount 4)
            (`KismetSystemLibrary.PrintString` "WINNER" true true (struct :`G` 0.66 :`B` 1.0 :`A` 1.0) 5.0)
            (bind _asblock (cast `Block` (`self.targetBlock`)))
            (set `Block.isActive` true _asblock)
            (`KismetSystemLibrary.Delay` 2.0)
            (bind _ascat_pickup_bp (cast `/Game/BOOOOOOOOprints/CatPickup_BP` (`self.targetCatPickup`)))
            (`SceneComponent.SetVisibility` (`/Game/BOOOOOOOOprints/CatPickup_BP.PaperSprite` _ascat_pickup_bp) true false)))))))

(event `self.CollisionComponent.OnComponentEndOverlap`
  (params (OverlappedComponent :type "PrimitiveComponent Object Reference") (OtherActor :type "Actor Object Reference") (OtherComp :type "PrimitiveComponent Object Reference") (OtherBodyIndex :type Integer))
  (bind _asdraggable_block (cast `DraggableBlock` OtherActor))
  (if (== OtherActor _asdraggable_block)
    (if (`DraggableBlock.isSpecial` _asdraggable_block)
      (`/Engine/EditorBlueprintResources/StandardMacros.DecrementInt` (`self.WinCount`)
        (:`  `
          (`KismetSystemLibrary.PrintString` "-1"))))))

(fn `UserConstructionScript`)